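; Melee player Blueprint that handles a telegraphed sword basic attack.
; Pressing BasicAttack spawns a sector telegraph attached to the mesh; releasing destroys it and plays the slash montage, gated by DoOnce for the montage's length.
; Trigger and stop sword events control a fast looping timer that line-traces between the sword's sockets with debug drawing, applying damage on every trace, so one swing can damage repeatedly.
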(event `InputAction|BasicAttack`
  (params (Key :type "Key Structure"))
  (bind _mesh (`self.Mesh`))
  (:`Pressed`
    (bind _returnvalue (`|SpawnActorFromClass` "/Game/EPOC_BP/VFX_/VFX_Decal/VFX_Actor_SectorSkill.VFX_Actor_SectorSkill_C" (`KismetMathLibrary.MakeTransform` (`SceneComponent.K2_GetComponentLocation` _mesh) (`SceneComponent.K2_GetComponentRotation` _mesh)) "Undefined" "OverrideRootScale" null null))
    (bind _output_get (set `self.sectorTelegraphRef` _returnvalue))
    (`self.K2_AttachToComponent` _output_get (`self.Mesh`) "None" "KeepWorld" "KeepWorld" "KeepWorld" true))
  (:`Released`
    (`self.K2_DestroyActor` (`self.sectorTelegraphRef`))
    (`/Engine/EditorBlueprintResources/StandardMacros.DoOnce` false :!label _label
      (:`Completed`
        (bind _returnvalue_2 (`self.PlayAnimMontage` "/Game/EPOC_BP/combatSystem/SwordSlash_Montage.SwordSlash_Montage"))
        (`KismetSystemLibrary.Delay` _returnvalue_2)
        (goto _label :!via `Reset`)))))

(event `triggerSword`
  (bind _returnvalue (`KismetSystemLibrary.K2_SetTimerDelegate` (delegate `swordLineTrace`) 0.01 true))
  (set `self.triggerSwordEvent` _returnvalue))

(event `swordLineTrace`
  (bind _sword (`self.sword`))
  (bind _outhit (`KismetSystemLibrary.LineTraceSingle` :`Start` (`SceneComponent.GetSocketLocation` _sword "start") :`End` (`SceneComponent.GetSocketLocation` _sword "end") :`TraceChannel` "TraceTypeQuery2" :`DrawDebugType` "ForDuration"))
  (`GameplayStatics.ApplyDamage` (`.HitActor` (`GameplayStatics.BreakHitResult` _outhit)) 1.0))

(event `stopTriggerSword`
  (`KismetSystemLibrary.K2_ClearAndInvalidateTimerHandle` (`self.triggerSwordEvent`)))

(fn `UserConstructionScript`
  (`parent.UserConstructionScript`))