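; Per-player input receiver that handles local join and character selection before the player is spawned.
; Outside of gameplay, Start asks the GameMode to display character select for its PlayerIndex, while MenuLeft and MenuRight cycle the open menu's character.
; With a menu open, Start has the GameMode spawn the chosen character, removes the menu and displays that player's status.
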(event `InputAction|Start`
  (params (Key :type "Key Structure"))
  (bind _characterchoice (`/Game/EPOC_BP/EPOC_CONTENT/Blueprints/UI/WBP_CharacterSelect.CharacterChoice` (`self.CharacterMenuRef`)))
  (:`Pressed`
    (bind _isingame (message `/Game/EPOC_BP/EPOC_CONTENT/Blueprints/BPI_GameMode.GetIsIngame` (`GameplayStatics.GetGameMode`)))
    (if (not _isingame)
      (`/Engine/EditorBlueprintResources/StandardMacros.IsValid` (`self.CharacterMenuRef`)
        (:`Is Valid`
          (message `/Game/EPOC_BP/EPOC_CONTENT/Blueprints/BPI_GameMode.SpawnPlayer` (`GameplayStatics.GetGameMode`) (`self.PlayerIndex`) _characterchoice self)
          (`Widget.RemoveFromParent` (`self.CharacterMenuRef`))
          (message `/Game/EPOC_BP/EPOC_CONTENT/Blueprints/BPI_GameMode.DisplayPlayerStatus` self _characterchoice))
        (:`Is Not Valid`
          (message `/Game/EPOC_BP/EPOC_CONTENT/Blueprints/BPI_GameMode.DisplayCharacterSelect` (`GameplayStatics.GetGameMode`) (`self.PlayerIndex`)))))))

(event `InputAction|MenuLeft`
  (params (Key :type "Key Structure"))
  (:`Pressed`
    (`/Engine/EditorBlueprintResources/StandardMacros.IsValid` (`self.CharacterMenuRef`)
      (:`Is Valid`
        (`/Game/EPOC_BP/EPOC_CONTENT/Blueprints/UI/WBP_CharacterSelect.SwitchCharacter` (`self.CharacterMenuRef`) -1)))))

(event `InputAction|MenuRight`
  (params (Key :type "Key Structure"))
  (:`Pressed`
    (`/Engine/EditorBlueprintResources/StandardMacros.IsValid` (`self.CharacterMenuRef`)
      (:`Is Valid`
        (`/Game/EPOC_BP/EPOC_CONTENT/Blueprints/UI/WBP_CharacterSelect.SwitchCharacter` (`self.CharacterMenuRef`) 1)))))

(fn `UserConstructionScript`)