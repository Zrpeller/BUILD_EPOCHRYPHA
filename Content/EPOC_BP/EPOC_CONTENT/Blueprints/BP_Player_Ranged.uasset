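; Ranged player Blueprint that implements a hold-and-release projectile basic attack.
; Pressing BasicAttack spawns a linear skill telegraph attached to the character and starts a looping timer calling IncreaseProjectileStrength by name.
; Releasing it stops the timer, removes the telegraph and fires a BP_Projectile from the SpawnProjectile transform.
; ProjectilePower serves as the projectile's lifetime through a Delay before destruction, then resets.
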(event `InputAction|BasicAttack`
  (params (Key :type "Key Structure"))
  (bind _mesh (`self.Mesh`))
  ;[1 1 1] Ranged Player Attacks
  (:`Pressed`
    (bind _returnvalue (`|SpawnActorFromClass` "/Game/EPOC_BP/VFX_/VFX_Decal/VFX_Actor_LinearSkill.VFX_Actor_LinearSkill_C" (`KismetMathLibrary.MakeTransform` (`SceneComponent.K2_GetComponentLocation` _mesh) (`SceneComponent.K2_GetComponentRotation` _mesh) (0.1 2.5 0.2)) "Undefined" "OverrideRootScale" null null))
    (bind _output_get (set `self.linearActorRef` _returnvalue))
    (`self.K2_AttachToComponent` _output_get (`self.LinerSkillTelegraphPoint`) "None" "KeepWorld" "KeepWorld" "KeepWorld" true)
    (bind _returnvalue_2 (`KismetSystemLibrary.K2_SetTimer` null "IncreaseProjectileStrength" 0.0 true)))
  (:`Released`
    (`KismetSystemLibrary.K2_ClearAndInvalidateTimerHandle` _returnvalue_2)
    (`self.K2_DestroyActor` (`self.linearActorRef`))
    (bind _returnvalue_3 (`|SpawnActorFromClass` "/Game/EPOC_BP/EPOC_CONTENT/Blueprints/BP_Projectile.BP_Projectile_C" (`SceneComponent.K2_GetComponentToWorld` (`self.SpawnProjectile`)) "Undefined" "OverrideRootScale" null null))
    (`KismetSystemLibrary.Delay` (`self.ProjectilePower`))
    (`self.K2_DestroyActor` _returnvalue_3)
    (set `self.ProjectilePower` 0.15)))

(fn `UserConstructionScript`
  (`parent.UserConstructionScript`))