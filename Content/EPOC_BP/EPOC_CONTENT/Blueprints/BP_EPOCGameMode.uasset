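; Game mode for local multiplayer that runs player setup, character selection and game start.
; On BeginPlay it creates players at PlayerStarts ordered by numeric tag, each possessing a BP_InputReceiver and viewing a shared BP_Camera, then shows WBP_Menu.
; SpawnPlayer swaps a receiver for the chosen ranged, melee or base character.
; StartGame requires a minimum player count, then sets the in-game flag and passes the players to the camera.
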(event `self.ReceiveBeginPlay`
  (`self.ActivateCamerasAndPlayers`))

(event `InputAction|StartGame`
  (params (Key :type "Key Structure"))
  (:`Pressed`
    (bind _returnvalue (`|CreateWidget` "/Game/EPOC_BP/EPOC_CONTENT/Blueprints/UI/WBP_PlayerHUD.WBP_PlayerHUD_C" null true))
    (bind _output_get (set `self.PlayerHUDRef` _returnvalue))
    (`UserWidget.AddToViewport` _output_get 0)))

(fn `ActivateCamerasAndPlayers`
  (bind _outactors (`GameplayStatics.GetAllActorsOfClass` "/Game/EPOC_BP/EPOC_CONTENT/Blueprints/BP_Camera.BP_Camera_C"))
  (set `self.CameraRef` (`|GetArrayItem` _outactors))
  (`self.Set Player Start Points`)
  (`self.SpawnInputReceivers`)
  (bind _returnvalue (`|CreateWidget` "/Game/EPOC_BP/EPOC_CONTENT/Blueprints/UI/WBP_Menu.WBP_Menu_C"))
  (bind _output_get (set `self.MenuWidgetRef` _returnvalue))
  (`UserWidget.AddToViewport` _output_get 0))

(fn `DisplayCharacterSelect`
  (params (CurrentPlayerIndex :type Integer))
  (returns (Return :type Boolean))
  (bind _characterselect (`/Game/EPOC_BP/EPOC_CONTENT/Blueprints/UI/WBP_Menu.AddCharacterSelect` (`self.MenuWidgetRef`) CurrentPlayerIndex))
  (set `/Game/EPOC_BP/EPOC_CONTENT/Blueprints/BP_InputReceiver.CharacterMenuRef` _characterselect (`|GetArrayItem` (`self.PlayerInputReceiverArray`) (`local.CurrentPlayerIndex`)))
  (return false))

(fn `DisplayPlayerStatus`
  (params (PlayerCharacterChoice :type Integer))
  (returns (Return :type Boolean))
  (bind _playerstatus (`/Game/EPOC_BP/EPOC_CONTENT/Blueprints/UI/WBP_PlayerHUD.AddPlayerToHUD` (`self.PlayerHUDRef`) PlayerCharacterChoice))
  (set `/Game/EPOC_BP/EPOC_CONTENT/Blueprints/BP_InputReceiver.PlayerStatusRef` _playerstatus (`|GetArrayItem` (`self.PlayerInputReceiverArray`) (`local.PlayerCharacterChoice`)))
  (return false))

(fn `GameStarted`
  (returns (OutputGameState :type Boolean))
  (bind _output_get (set `self.bIsInGame` true))
  (`/Game/EPOC_BP/EPOC_CONTENT/Blueprints/BP_Camera.GameStarted` (`self.CameraRef`) (`self.Players`))
  (return _output_get))

(fn `GetIsIngame`
  (returns (IsInGame :type Boolean))
  (return (`self.bIsInGame`)))

(fn `NameToInt`
  (params (PlayerStart :type "PlayerStart Object Reference"))
  (returns (ReturnValue :type Integer))
  (return (`KismetStringLibrary.Conv_StringToInt` (`KismetStringLibrary.Conv_NameToString` (`PlayerStart.PlayerStartTag` PlayerStart)))))

(fn `RemoveUnusedCamera`
  (bind _outactors (`GameplayStatics.GetAllActorsOfClass` "/Script/Engine.CameraActor"))
  (for _array_element _outactors
    (`self.K2_DestroyActor` _array_element)))

(fn `Set Player Start Points`
  (bind _outactors (`GameplayStatics.GetAllActorsOfClass` "/Script/Engine.PlayerStart"))
  (set `self.PlayerStartArray` _outactors))

(fn `SpawnInputReceivers`
  (locals (Index :type Integer))
  (bind _returnvalue (`GameplayStatics.GetPlayerController` (`local.Index`)))
  (for (_ _array_index) (`self.PlayerStartArray`)
    (set `local.Index` _array_index)
    (for _array_element (`self.PlayerStartArray`)
      (if (== (`self.NameToInt` _array_element) (`local.Index`))
        (`GameplayStatics.CreatePlayer` -1)
        (bind _returnvalue_2 (`|SpawnActorFromClass` "/Game/EPOC_BP/EPOC_CONTENT/Blueprints/BP_InputReceiver.BP_InputReceiver_C" (`self.GetTransform` (`|GetArrayItem` (`self.PlayerStartArray`) (`local.Index`))) "Undefined" "OverrideRootScale" null (`local.Index`) null))
        (`KismetArrayLibrary.Array_AddUnique` (`self.PlayerInputReceiverArray`) _returnvalue_2)
        (`Controller.Possess` _returnvalue _returnvalue_2)
        (`KismetArrayLibrary.Array_AddUnique` (`self.PlayerControllerArray`) _returnvalue)
        (`PlayerController.SetViewTargetWithBlend` (`GameplayStatics.GetPlayerController` (`local.Index`)) (`self.CameraRef`) 0.0 "VTBlend_Linear" 0.0 false)))
    (`self.RemoveUnusedCamera`)))

(fn `SpawnPlayer`
  (params (CurrentPlayerIndex :type Integer) (CharacterChoice :type Integer) (InputReciever :type "/Game/EPOC_BP/EPOC_CONTENT/Blueprints/BP_InputReceiver Object Reference"))
  (returns (Return :type Boolean))
  (if (== CharacterChoice 0)
    (bind _returnvalue (`|SpawnActorFromClass` "/Game/EPOC_BP/EPOC_CONTENT/Blueprints/BP_Player_Ranged.BP_Player_Ranged_C" (`self.GetTransform` (`local.InputReciever`)) "Undefined" "OverrideRootScale" null CharacterChoice 0.15 null))
    (`KismetArrayLibrary.Array_Add` (`self.Players`) _returnvalue)
    (`Controller.Possess` (`GameplayStatics.GetPlayerController` (`local.CurrentPlayerIndex`)) _returnvalue)
    (`PlayerController.SetViewTargetWithBlend` (`GameplayStatics.GetPlayerController` (`local.CurrentPlayerIndex`)) (`self.CameraRef`) 0.0 "VTBlend_Linear" 0.0 false)
    (return false)
    (elif (== CharacterChoice 1)
      (bind _returnvalue_2 (`|SpawnActorFromClass` "/Game/EPOC_BP/EPOC_CONTENT/Blueprints/BP_Player_Melee.BP_Player_Melee_C" (`self.GetTransform` (`local.InputReciever`)) "Undefined" "OverrideRootScale" null CharacterChoice 0.15 null))
      (`KismetArrayLibrary.Array_Add` (`self.Players`) _returnvalue_2)
      (`Controller.Possess` (`GameplayStatics.GetPlayerController` (`local.CurrentPlayerIndex`)) _returnvalue_2)
      (`PlayerController.SetViewTargetWithBlend` (`GameplayStatics.GetPlayerController` (`local.CurrentPlayerIndex`)) (`self.CameraRef`) 0.0 "VTBlend_Linear" 0.0 false)
      (return false)
      (elif (== CharacterChoice 2)
        (bind _returnvalue_3 (`|SpawnActorFromClass` "/Game/EPOC_BP/EPOC_CONTENT/Blueprints/BP_Player.BP_Player_C" (`self.GetTransform` (`local.InputReciever`)) "Undefined" "OverrideRootScale" null CharacterChoice 0.15 null))
        (`KismetArrayLibrary.Array_Add` (`self.Players`) _returnvalue_3)
        (`Controller.Possess` (`GameplayStatics.GetPlayerController` (`local.CurrentPlayerIndex`)) _returnvalue_3)
        (`PlayerController.SetViewTargetWithBlend` (`GameplayStatics.GetPlayerController` (`local.CurrentPlayerIndex`)) (`self.CameraRef`) 0.0 "VTBlend_Linear" 0.0 false)
        (return false)))))

(fn `StartGame`
  (returns (Return :type Boolean))
  (if (>= (`KismetArrayLibrary.Array_Length` (`self.Players`)) (`self.minimumPlayers`))
    (`|CreateWidget` "/Game/EPOC_BP/EPOC_CONTENT/Blueprints/UI/WBP_PlayerHUD.WBP_PlayerHUD_C" null true)
    (`self.GameStarted`)
    (return false)))

(fn `UserConstructionScript`)